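; BP_Player is the player Blueprint that turns left and right flipper input into actions on the bats in the level.
; On BeginPlay it adds the IMC_Player Enhanced Input mapping context and caches all BP_Left_Bat and BP_Right_Bat actors into two arrays.
; Each flipper input action loops over its side's array and calls TriggerMessage on every bat, leaving the response to the bats.
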(event `self.ReceiveBeginPlay`
  (`EnhancedInputSubsystemInterface.AddMappingContext` (pcsubsystem `EnhancedInputLocalPlayerSubsystem` (`GameplayStatics.GetPlayerController` 0)) "/Game/Blueprints/Input/IMC_Player.IMC_Player" 0 (struct))
  (bind _outactors (`GameplayStatics.GetAllActorsOfClass` "/Game/Blueprints/BP_Left_Bat.BP_Left_Bat_C"))
  (set `self.LeftBats` _outactors)
  (bind _outactors_2 (`GameplayStatics.GetAllActorsOfClass` "/Game/Blueprints/BP_Right_Bat.BP_Right_Bat_C"))
  (set `self.RightBats` _outactors_2))

(event `EnhancedInput|/Game/Blueprints/Input/IA_LeftFlipper`
  (params (ActionValue :type Boolean) (ElapsedSeconds :type "Float (double-precision)") (TriggeredSeconds :type "Float (double-precision)") (InputAction :type "InputAction Object Reference" :default "/Game/Blueprints/Input/IA_LeftFlipper.IA_LeftFlipper"))
  (:`Triggered`
    (for _array_element (`self.LeftBats`)
      (message `/Game/Blueprints/BPI_Bat_Actions.Trigger` _array_element))))

(event `EnhancedInput|/Game/Blueprints/Input/IA_RightFlipper`
  (params (ActionValue :type Boolean) (ElapsedSeconds :type "Float (double-precision)") (TriggeredSeconds :type "Float (double-precision)") (InputAction :type "InputAction Object Reference" :default "/Game/Blueprints/Input/IA_RightFlipper.IA_RightFlipper"))
  (:`Triggered`
    (for _array_element (`self.RightBats`)
      (message `/Game/Blueprints/BPI_Bat_Actions.Trigger` _array_element))))

(fn `UserConstructionScript`)