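; BP_Machine is the ball game's table actor, reporting ball and launcher zone events to BP_Player.
; On BeginPlay it caches all BP_Player actors and adds the WB_ScoreBoard widget to the viewport.
; DestroyBallBox overlaps play a lost-ball sound and pass the BP_Ball to LostBall.
; LaunchZone overlaps toggle the players' launch-zone state, while leaving GateZoneLauncher calls CloseLaunchGate on the last cached player.
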(event `self.ReceiveBeginPlay`
  (bind _outactors (`GameplayStatics.GetAllActorsOfClass` "/Game/Blueprints/Framework/BP_Player.BP_Player_C"))
  (set `self.PlayerRef` _outactors)
  (bind _returnvalue (`|CreateWidget` "/Game/UI/WB_ScoreBoard.WB_ScoreBoard_C" (`GameplayStatics.GetPlayerController` 0)))
  (`UserWidget.AddToViewport` _returnvalue 0))

(event `self.Destroy Ball Box.OnComponentBeginOverlap`
  (params (OverlappedComponent :type "PrimitiveComponent Object Reference") (OtherActor :type "Actor Object Reference") (OtherComp :type "PrimitiveComponent Object Reference") (OtherBodyIndex :type Integer) (bFromSweep :type Boolean) (SweepResult :type "HitResult Structure (by ref)"))
  (`GameplayStatics.PlaySound2D` "/Game/Sounds/BallLost.BallLost" 1.0 1.0 0.0 null null)
  (bind _asbp_ball (cast `/Game/Blueprints/BP_Ball` OtherActor))
  (`/Game/Blueprints/Framework/BP_Player.LostBall` (`self.PlayerRef`) _asbp_ball))

(event `self.LaunchZone.OnComponentBeginOverlap`
  (params (OverlappedComponent :type "PrimitiveComponent Object Reference") (OtherActor :type "Actor Object Reference") (OtherComp :type "PrimitiveComponent Object Reference") (OtherBodyIndex :type Integer) (bFromSweep :type Boolean) (SweepResult :type "HitResult Structure (by ref)"))
  (`/Game/Blueprints/Framework/BP_Player.InLaunchZone` (`self.PlayerRef`) true))

(event `self.LaunchZone.OnComponentEndOverlap`
  (params (OverlappedComponent :type "PrimitiveComponent Object Reference") (OtherActor :type "Actor Object Reference") (OtherComp :type "PrimitiveComponent Object Reference") (OtherBodyIndex :type Integer))
  (`/Game/Blueprints/Framework/BP_Player.InLaunchZone` (`self.PlayerRef`) false))

(event `self.GateZoneLauncher.OnComponentEndOverlap`
  (params (OverlappedComponent :type "PrimitiveComponent Object Reference") (OtherActor :type "Actor Object Reference") (OtherComp :type "PrimitiveComponent Object Reference") (OtherBodyIndex :type Integer))
  (bind _playerref (`self.PlayerRef`))
  (`/Game/Blueprints/Framework/BP_Player.CloseLaunchGate` (`|GetArrayItem` _playerref (`KismetArrayLibrary.Array_LastIndex` _playerref)) true))

(fn `UserConstructionScript`)