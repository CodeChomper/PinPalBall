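; BP_Ball is a physics ball launched by a hold-and-release charge.
; Trigger starts a recursive delayed Charging loop that steadily drives LaunchPower negative to a clamped limit, printing it as debug output.
; Released stops the loop, applies the power as an X-axis impulse to the Sphere and resets it.
; Tick caps the Sphere's linear velocity by clamping its vector size.
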(event `self.ReceiveTick`
  (params (DeltaSeconds :type "Float (single-precision)"))
  (bind _sphere (`self.Sphere`))
  (bind _returnvalue (`PrimitiveComponent.GetPhysicsLinearVelocity` _sphere "None"))
  (`PrimitiveComponent.SetPhysicsLinearVelocity` _sphere (`KismetMathLibrary.ClampVectorSize` _returnvalue -300.0 300.0) false "None"))

(event `Charging`
  (if (stale `/Game/Blueprints/BPI_Launcher.Trigger` _output_get) :!label _label
    (bind _output_get (set `self.LaunchPower` (`KismetMathLibrary.FClamp` (+ (`self.LaunchPower`) -0.15) -30.0 0.0)))
    (`KismetSystemLibrary.Delay` 0.007)
    (`KismetSystemLibrary.PrintString` (`KismetStringLibrary.Conv_DoubleToString` _output_get))
    (`self.Charging`)))

(event `/Game/Blueprints/BPI_Launcher.Trigger`
  (bind _output_get (set `self.Launching?` true))
  (goto _label))

(event `/Game/Blueprints/BPI_Launcher.Released`
  (set `self.Launching?` false)
  (`PrimitiveComponent.AddImpulse` (`self.Sphere`) (`KismetMathLibrary.MakeVector` (`self.LaunchPower`)) "None" false)
  (`KismetSystemLibrary.PrintString` "LAUNCHED!")
  (set `self.LaunchPower` 0.0))

(fn `UserConstructionScript`)