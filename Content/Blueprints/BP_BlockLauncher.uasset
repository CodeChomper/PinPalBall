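; BP_BlockLauncher is a pinball-style blocker actor that raises Blocker001 again after a timed stay down.
; LiftUp reverses the GoingDown timeline to drive the blocker's relative Z, and the timeline's Finished output sets a timer to call LiftUp.
; An unconnected chain, which never runs, holds the BP_Ball hit response: impulse, audio and a hit counter that plays the drop on the third hit.
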(event `LiftUp`
  (bind (_direction _zval) (`Timeline|GoingDown` :!via `ReverseFromEnd`)
    (:`Update`
      (`SceneComponent.K2_SetRelativeLocation` (`self.Blocker_001`) (`KismetMathLibrary.MakeVector` 0.0 0.0 _zval) false false))
    (:`Finished`
      (`KismetSystemLibrary.K2_SetTimer` null "LiftUp" (`self.SecondsToStayDown`)))))

(fn `UserConstructionScript`)