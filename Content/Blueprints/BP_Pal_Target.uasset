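; BP_Pal_Target is a sprite target that advances at random intervals and costs the player score while at its furthest step.
; A repeating random timer raises the step count, and Tick lerps the child actor toward that offset.
; A BP_Ball hit resets the steps and plays the Laydown timeline, reversed after a delay to stand back up.
; Points accrue on every timeline update, so both falling and rising add score.
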(event `StepForward`
  (if (and (> (`KismetMathLibrary.RandomIntegerInRange` 0 1) 0) (< (`self.StepsForward`) 6))
    (`/Engine/EditorBlueprintResources/StandardMacros.IncrementInt` (`self.StepsForward`)
      (:`  `
        _)))
  (`KismetSystemLibrary.K2_SetTimer` null "StepForward" (`KismetMathLibrary.Conv_IntToDouble` (`KismetMathLibrary.RandomIntegerInRange` 2 4)))
  (if (>= (`self.StepsForward`) 6)
    (`/Game/Blueprints/Framework/BP_Player.AddToScore` (`self.PlayerRef`) -50)))

(event `self.ReceiveBeginPlay`
  (`KismetSystemLibrary.K2_SetTimer` null "StepForward" 10.0)
  (bind _outactors (`GameplayStatics.GetAllActorsOfClass` "/Game/Blueprints/Framework/BP_Player.BP_Player_C"))
  (set `self.PlayerRef` (`|GetArrayItem` _outactors (`KismetArrayLibrary.Array_LastIndex` _outactors))))

(event `self.ReceiveTick`
  (params (DeltaSeconds :type "Float (single-precision)"))
  (`SceneComponent.K2_SetRelativeLocation` (`self.ChildActor`) (`KismetMathLibrary.MakeVector` (`KismetMathLibrary.Lerp` (.x (.location (`SceneComponent.GetRelativeTransform` (`self.ChildActor`)))) (`KismetMathLibrary.Conv_IntToDouble` (* (`self.StepsForward`) 5)) DeltaSeconds) 0.0 0.151565) true false))

(event `self.pal_01_Sprite.OnComponentHit`
  (params (HitComponent :type "PrimitiveComponent Object Reference") (OtherActor :type "Actor Object Reference") (OtherComp :type "PrimitiveComponent Object Reference") (NormalImpulse :type "Vector Structure") (Hit :type "HitResult Structure (by ref)"))
  (cast `/Game/Blueprints/BP_Ball` OtherActor)
  (`KismetSystemLibrary.K2_SetTimer` null "StandBackUp" 2.0)
  (set `self.StepsForward` 0)
  (bind (_direction _newtrack_0) (`Timeline|Laydown` :!label _label)
    (:`Update`
      (`SceneComponent.K2_SetRelativeRotation` (`self.ChildActor`) (`KismetMathLibrary.MakeRotator` 0.0 _newtrack_0) false false)
      (`/Game/Blueprints/Framework/BP_Player.AddToScore` (`self.PlayerRef`) 1))))

(event `StandBackUp`
  (goto _label :!via `ReverseFromEnd`))

(fn `UserConstructionScript`
  (`PaperSpriteComponent.SetSprite` (`self.pal_01_Sprite`) (`self.Sprite`)))