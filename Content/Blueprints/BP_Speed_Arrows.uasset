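; BP_Speed_Arrows is a boost pad that speeds up a BP_Ball passing over it.
; Either of two box triggers calls BoostSpeed, which plays a sound and applies an impulse scaled from the ball's current linear velocity, so the boost follows its direction of travel.
; A CanBoost flag, reset by a timer calling CoolDown, blocks repeat boosts for a few seconds.
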(event `self.Box1.OnComponentBeginOverlap`
  (params (OverlappedComponent :type "PrimitiveComponent Object Reference") (OtherActor :type "Actor Object Reference") (OtherComp :type "PrimitiveComponent Object Reference") (OtherBodyIndex :type Integer) (bFromSweep :type Boolean) (SweepResult :type "HitResult Structure (by ref)"))
  (bind _asbp_ball (cast `/Game/Blueprints/BP_Ball` OtherActor))
  (`self.Boost Speed` _asbp_ball))

(event `Boost Speed`
  (params (Ball :type "/Game/Blueprints/BP_Ball Object Reference"))
  (bind _sphere (`/Game/Blueprints/BP_Ball.Sphere` Ball))
  (if (`self.CanBoost`)
    (set `self.CanBoost` false)
    (`AudioComponent.Play` (`self.Audio`) 0.0)
    (bind _returnvalue (`PrimitiveComponent.GetPhysicsLinearVelocity` _sphere "None"))
    (`PrimitiveComponent.AddImpulse` _sphere (* _returnvalue 1.2) "None" false)
    (`KismetSystemLibrary.K2_SetTimer` null "Cooldown" 3.0)))

(event `self.Box.OnComponentBeginOverlap`
  (params (OverlappedComponent :type "PrimitiveComponent Object Reference") (OtherActor :type "Actor Object Reference") (OtherComp :type "PrimitiveComponent Object Reference") (OtherBodyIndex :type Integer) (bFromSweep :type Boolean) (SweepResult :type "HitResult Structure (by ref)"))
  (bind _asbp_ball (cast `/Game/Blueprints/BP_Ball` OtherActor))
  (`self.Boost Speed` _asbp_ball))

(event `CoolDown`
  (set `self.CanBoost` true))

(fn `UserConstructionScript`)