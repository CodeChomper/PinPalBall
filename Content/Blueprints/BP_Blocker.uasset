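; BP_Blocker is an obstacle that knocks a BP_Ball away when hit and temporarily lowers after repeated hits.
; Each ball hit applies the normal impulse to the ball's sphere, plays audio and advances a hit counter.
; Once the counter exceeds one, it resets and the GoingDown timeline moves the blocker mesh along Z.
; When the timeline finishes, a timer calls LiftUp after SecondsToStayDown, reversing the timeline.
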(event `self.Blocker_001.OnComponentHit`
  (params (HitComponent :type "PrimitiveComponent Object Reference") (OtherActor :type "Actor Object Reference") (OtherComp :type "PrimitiveComponent Object Reference") (NormalImpulse :type "Vector Structure") (Hit :type "HitResult Structure (by ref)"))
  (bind _asbp_ball (cast `/Game/Blueprints/BP_Ball` OtherActor))
  (`PrimitiveComponent.AddImpulse` (`/Game/Blueprints/BP_Ball.Sphere` _asbp_ball) NormalImpulse "None" false)
  (`AudioComponent.Play` (`self.Audio`) 0.0)
  (if (> (`self.NumberOfHits`) 1)
    (set `self.NumberOfHits` 0)
    (bind (_direction _zval) (`Timeline|GoingDown` :!label _label)
      (:`Update`
        (`SceneComponent.K2_SetRelativeLocation` (`self.Blocker_001`) (`KismetMathLibrary.MakeVector` 0.0 0.0 _zval) false false))
      (:`Finished`
        (`KismetSystemLibrary.K2_SetTimer` null "LiftUp" (`self.SecondsToStayDown`))))
    (else
      (`/Engine/EditorBlueprintResources/StandardMacros.IncrementInt` (`self.NumberOfHits`)))))

(event `LiftUp`
  (goto _label :!via `ReverseFromEnd`))

(fn `UserConstructionScript`)